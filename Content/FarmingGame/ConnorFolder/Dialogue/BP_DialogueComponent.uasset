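; Dialogue component that steps through data-table-driven conversations, one line per Talk call.
; The first call locks the first-person character's camera and creates the dialogue widget with the speaker name and line.
; Each row supplies the next row, table and end flag, chaining lines across tables.
; Later calls update the widget, unlock the camera and hide the cursor; once the end flag is set, the next call removes the widget.
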(event `/Game/FarmingGame/ConnorFolder/Dialogue/BP_Talk.Talk`
  (params (playerRef :type "/Game/FirstPerson/Blueprints/BP_FirstPersonCharacter Object Reference"))
  ; Trigger dialogue
  (if (`self.EndDialogue`)
    ; End dialogue
    (`Widget.RemoveFromParent` (`self.DialogueWidget`))
    (set `self.EndDialogue` false)
    (set `self.DialogueWidget` null)
    (else
      (bind _asbp_first_person_character (cast `/Game/FirstPerson/Blueprints/BP_FirstPersonCharacter` (`GameplayStatics.GetPlayerCharacter` 0)))
      (set `/Game/FirstPerson/Blueprints/BP_FirstPersonCharacter.cameraLock` true _asbp_first_person_character)
      (`/Engine/EditorBlueprintResources/StandardMacros.IsValid` (`self.DialogueWidget`)
        (:`Is Valid`
          ; Update dialogue
          (bind _returnvalue (`|GetDataTableRow` (`self.Data Table`) (`self.Row Name`))
            (:`then`
              (bind (_dialogue _row _datetable _enddialogue) (break `/Game/FarmingGame/ConnorFolder/Dialogue/Dialogue_Structure` _returnvalue))
              (`/Game/FarmingGame/ConnorFolder/Dialogue/WidgetBlueprint_Dialogue.UpdateDialogue` (`self.DialogueWidget`) _dialogue)
              (set `self.Row Name` _row)
              (set `self.Data Table` _datetable)
              (set `self.EndDialogue` _enddialogue)
              (bind _asbp_first_person_character_2 (cast `/Game/FirstPerson/Blueprints/BP_FirstPersonCharacter` (`GameplayStatics.GetPlayerCharacter` 0)))
              (set `/Game/FirstPerson/Blueprints/BP_FirstPersonCharacter.cameraLock` false _asbp_first_person_character_2)
              (set `PlayerController.bShowMouseCursor` false (`GameplayStatics.GetPlayerController` 0)))))
        (:`Is Not Valid`
          (bind _returnvalue_2 (`|GetDataTableRow` (`self.Data Table`) (`self.Row Name`))
            (:`then`
              (bind (_dialogue_2 _row_2 _datetable_2 _enddialogue_2) (break `/Game/FarmingGame/ConnorFolder/Dialogue/Dialogue_Structure` _returnvalue_2))
              (bind _returnvalue_3 (`|CreateWidget` "/Game/FarmingGame/ConnorFolder/Dialogue/WidgetBlueprint_Dialogue.WidgetBlueprint_Dialogue_C" null (`KismetTextLibrary.Conv_NameToText` (`self.Name`)) _dialogue_2))
              (bind _output_get (set `self.DialogueWidget` _returnvalue_3))
              (`UserWidget.AddToViewport` _output_get 0)
              (set `self.Row Name` _row_2)
              (set `self.Data Table` _datetable_2)
              (set `self.EndDialogue` _enddialogue_2))))))))