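; EggBP is a collectible egg actor in the farming game that the player picks up by interacting with it.
; Interact increments CurrentEggs on FarmingGameInstance_BP, then creates a CurrentEggWidget showing the new total.
; After a short delay it removes the widget and destroys the egg, so the actor stays in the world while the popup displays.
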(event `self.ReceiveBeginPlay`)

(event `/Game/FarmingGame/CaraFolder/Interactable_BPI.Interact`
  (bind _asfarming_game_instance_bp (cast `/Game/FarmingGame/FarmingGameInstance_BP` (`GameplayStatics.GetGameInstance`)))
  (bind _output_get (set `/Game/FarmingGame/FarmingGameInstance_BP.currentEggs` (+ (`/Game/FarmingGame/FarmingGameInstance_BP.currentEggs` _asfarming_game_instance_bp) 1) _asfarming_game_instance_bp))
  (bind _returnvalue (`|CreateWidget` "/Game/FarmingGame/ConnorFolder/UIWidgets/CurrentEggWidget.CurrentEggWidget_C" (`GameplayStatics.GetPlayerController` 0)))
  (bind _output_get_2 (set `self.eggsWidget` _returnvalue))
  (`/Game/FarmingGame/ConnorFolder/UIWidgets/CurrentEggWidget.SupplyEggAmount` _output_get_2 (`KismetStringLibrary.Conv_IntToString` _output_get))
  (`UserWidget.AddToViewport` _output_get_2 0)
  (`KismetSystemLibrary.Delay` 1.0)
  (`Widget.RemoveFromParent` (`self.eggsWidget`))
  (`self.K2_DestroyActor`))

(fn `UserConstructionScript`)