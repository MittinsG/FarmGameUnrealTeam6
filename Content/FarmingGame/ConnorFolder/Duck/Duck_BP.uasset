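; Duck AI pawn for the farming game that can wander and notice the player.
; The Roaming event moves it to a random reachable point around its current location.
; When PawnSensing sees the first-person player character, it sets the WillFollow blackboard key on the duck's controller.
; FollowPlayer is an empty stub, and the direct move-to-player logic is left disconnected.
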(event `Roaming`
  (`|AIMoveTo` self (`NavigationSystemV1.K2_GetRandomReachablePointInRadius` (`self.K2_GetActorLocation`) 1000.0 null null) null))

(event `self.PawnSensing.OnSeePawn`
  (params (Pawn :type "Pawn Object Reference"))
  (cast `/Game/FirstPerson/Blueprints/BP_FirstPersonCharacter` Pawn)
  (`BlackboardComponent.SetValueAsBool` (`AIBlueprintHelperLibrary.GetBlackboard` (`self.GetController`)) "WillFollow" true))

(event `FollowPlayer`
  (if (`self.canSeePlayer`)
    _))

(fn `UserConstructionScript`)