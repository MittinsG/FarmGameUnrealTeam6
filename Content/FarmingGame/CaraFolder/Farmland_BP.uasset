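; Farmland Blueprint for a farming game that reports the state of a crop plot through debug print messages.
; On BeginPlay it runs a FarmlandCheck event, which branches on HasPlant, IsPlantGrown and HasSeed to print whether the crop is harvestable, still growing or seed can be placed.
; An Interact event only prints a confirmation; no planting, growth or harvest logic exists in this graph.
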(event `self.ReceiveBeginPlay`
  (`self.FarmlandCheck`))

(event `FarmlandCheck`
  (if (`self.HasPlant`)
    (if (`self.IsPlantGrown`)
      (`KismetSystemLibrary.PrintString` "The crop is harvestable")
      (else
        (`KismetSystemLibrary.PrintString` "The crop is still growing")))
    (elif (`self.HasSeed`)
      (`KismetSystemLibrary.PrintString` "Can Place seed")
      (else
        (`KismetSystemLibrary.PrintString` "You cant place a seed")))))

(event `/Game/FarmingGame/CaraFolder/Interactable_BPI.Interact`
  (`KismetSystemLibrary.PrintString` "Interacted"))

(fn `UserConstructionScript`)