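; Automatic gate actor that swings open when the first-person player enters either of its two trigger volumes and closes behind them.
; The front and back triggers set the swing direction, so the gate rotates 90 degrees one way or the other depending on the side entered.
; A timeline lerps the mesh rotation and plays in reverse to close, only once the player is clear of both triggers.
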(event `OpenGate`
  (if (`self.IsOpen`)
    _
    (elif (not (not (or (`KismetArrayLibrary.Array_Contains` (`PrimitiveComponent.GetOverlappingActors` (`self.FrontTrigger`) null) (`GameplayStatics.GetPlayerCharacter` 0)) (`KismetArrayLibrary.Array_Contains` (`PrimitiveComponent.GetOverlappingActors` (`self.BackTrigger`) null) (`GameplayStatics.GetPlayerCharacter` 0)))))
      ;[1 0.3315 0.07882 0.5] Sets the Rotation
      (if (`self.Reverse`)
        (set `self.OpenRotation` (`KismetMathLibrary.MakeRotator` 0.0 0.0 -90.0))
        (else
          (set `self.OpenRotation` (`KismetMathLibrary.MakeRotator` 0.0 0.0 90.0))))
      (set `self.IsOpen` true)
      ;[1 0.3315 0.07882 0.5] Rotation for the gate + Timeline
      (bind (_direction _alpha) (`Timeline|GateTimeline` :!label _label)
        (:`Update`
          (`SceneComponent.K2_SetRelativeRotation` (`self.GateMesh`) (`KismetMathLibrary.RLerp` (`self.ClosedRotation`) (`self.OpenRotation`) _alpha) false false))))))

(event `CloseGate`
  (if (`self.IsOpen`)
    (if (not (or (`KismetArrayLibrary.Array_Contains` (`PrimitiveComponent.GetOverlappingActors` (`self.FrontTrigger`) null) (`GameplayStatics.GetPlayerCharacter` 0)) (`KismetArrayLibrary.Array_Contains` (`PrimitiveComponent.GetOverlappingActors` (`self.BackTrigger`) null) (`GameplayStatics.GetPlayerCharacter` 0))))
      (set `self.IsOpen` false)
      (goto _label :!via `Reverse`))))

(event `self.FrontTrigger.OnComponentBeginOverlap`
  (params (OverlappedComponent :type "PrimitiveComponent Object Reference") (OtherActor :type "Actor Object Reference") (OtherComp :type "PrimitiveComponent Object Reference") (OtherBodyIndex :type Integer) (bFromSweep :type Boolean) (SweepResult :type "HitResult Structure (by ref)"))
  ;[1 0.3315 0.07882 0.5] Front Trigger
  (cast `/Game/FirstPerson/Blueprints/BP_FirstPersonCharacter` OtherActor)
  (set `self.Reverse` false)
  (`self.OpenGate`))

(event `self.FrontTrigger.OnComponentEndOverlap`
  (params (OverlappedComponent :type "PrimitiveComponent Object Reference") (OtherActor :type "Actor Object Reference") (OtherComp :type "PrimitiveComponent Object Reference") (OtherBodyIndex :type Integer))
  ;[1 0.3315 0.07882 0.5] Front Trigger
  (cast `/Game/FirstPerson/Blueprints/BP_FirstPersonCharacter` OtherActor)
  (`self.CloseGate`))

(event `self.BackTrigger.OnComponentBeginOverlap`
  (params (OverlappedComponent :type "PrimitiveComponent Object Reference") (OtherActor :type "Actor Object Reference") (OtherComp :type "PrimitiveComponent Object Reference") (OtherBodyIndex :type Integer) (bFromSweep :type Boolean) (SweepResult :type "HitResult Structure (by ref)"))
  ;[1 0.3315 0.07882 0.5] Back Trigger
  (cast `/Game/FirstPerson/Blueprints/BP_FirstPersonCharacter` OtherActor)
  (set `self.Reverse` true)
  (`self.OpenGate`))

(event `self.BackTrigger.OnComponentEndOverlap`
  (params (OverlappedComponent :type "PrimitiveComponent Object Reference") (OtherActor :type "Actor Object Reference") (OtherComp :type "PrimitiveComponent Object Reference") (OtherBodyIndex :type Integer))
  ;[1 0.3315 0.07882 0.5] Back Trigger
  (cast `/Game/FirstPerson/Blueprints/BP_FirstPersonCharacter` OtherActor)
  (`self.CloseGate`))

(fn `UserConstructionScript`)