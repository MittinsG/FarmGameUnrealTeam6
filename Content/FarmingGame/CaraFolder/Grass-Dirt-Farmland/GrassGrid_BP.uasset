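; GrassGrid_BP lays out a grid of grass child actors when constructed, with no active event graph logic.
; The construction script destroys the actors in SpawnedGrass and resets the array, then loops over GridSize X and Y.
; Each cell adds a child actor component offset by Spacing at a fixed height and records its actor in SpawnedGrass.
; The relative transform of each component also adds the grid actor's world location.
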(fn `UserConstructionScript`
  (for _array_element (`self.SpawnedGrass`)
    (`self.K2_DestroyActor` _array_element))
  (set `self.SpawnedGrass` (`|MakeArray` null :!type "Actor Object Reference"))
  (for _index (range (+ (`KismetMathLibrary.FTrunc` (- (.x (`self.GridSize`)) 1.0)) 1))
    (for _index_2 (range (+ (`KismetMathLibrary.FTrunc` (- (.y (`self.GridSize`)) 1.0)) 1))
      (bind _returnvalue (`AddComponent|NODE_AddChildActorComponent-0` :`RelativeTransform` (`KismetMathLibrary.MakeTransform` (+ (`KismetMathLibrary.MakeVector` (* (`KismetMathLibrary.Conv_IntToDouble` _index) (`self.Spacing`)) (* (`KismetMathLibrary.Conv_IntToDouble` _index_2) (`self.Spacing`)) 15.0) (`self.K2_GetActorLocation`)))))
      (`KismetArrayLibrary.Array_Add` (`self.SpawnedGrass`) (`ChildActorComponent.ChildActor` _returnvalue)))))