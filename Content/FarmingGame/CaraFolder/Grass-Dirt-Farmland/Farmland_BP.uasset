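; Farmland plot actor that takes a seed, grows a crop and yields a harvest, driven by a FarmlandState of Empty, Growing or Harvestable.
; Tool interaction plants seed items, removing them from the hotbar and spawning a Crop_BP.
; A looping timer, paced by the seed's growth time and stage count, advances progress in fixed increments and updates the crop's stage.
; Harvesting requires the hoe, spawns the seed's harvest item and resets the plot.
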(event `/Game/FarmingGame/AnthonyFolder/BPI_ItemAction.OnToolInteract`
  (params (ItemData :type "/Game/FarmingGame/AnthonyFolder/Items/ItemBP/BP_BaseItem Class Reference") (Inventory :type "/Game/FarmingGame/AnthonyFolder/BPC_Inventory Object Reference"))
  (set `self.Inventory` Inventory)
  (switch `/Game/FarmingGame/CaraFolder/Grass-Dirt-Farmland/EPlotState` (`self.FarmlandState`)
    (:`NewEnumerator0`
      (`self.Plant` ItemData))
    (:`NewEnumerator2`
      (`self.Harvest` ItemData))))

(event `Plant`
  (params (ItemData :type "/Game/FarmingGame/AnthonyFolder/Items/ItemBP/BP_BaseItem Class Reference"))
  (bind (_growthtime _growthstagemeshes) (defaults `Object` (`self.CurrentSeed`)))
  (if (`KismetMathLibrary.ClassIsChildOf` ItemData "/Game/FarmingGame/AnthonyFolder/Items/ItemBP/BP_Item_Seeds.BP_Item_Seeds_C")
    (bind _asbp_item_seeds (castclass `/Game/FarmingGame/AnthonyFolder/Items/ItemBP/BP_Item_Seeds` ItemData))
    (set `self.CurrentSeed` (defaults `Object` _asbp_item_seeds))
    (set `self.FarmlandState` "NewEnumerator1")
    (set `self.GrowthProgress` 0.0)
    (`/Game/FarmingGame/AnthonyFolder/BPC_Inventory.RemoveItemFromHotbar` (`self.Inventory`) false)
    (bind _returnvalue (`|SpawnActorFromClass` "/Game/FarmingGame/CaraFolder/Grass-Dirt-Farmland/Crop_BP.Crop_BP_C" (`self.GetTransform`) "Undefined" "MultiplyWithRoot" null null))
    (set `/Game/FarmingGame/CaraFolder/Grass-Dirt-Farmland/Crop_BP.SeedData` (`self.CurrentSeed`) _returnvalue)
    (`/Game/FarmingGame/CaraFolder/Grass-Dirt-Farmland/Crop_BP.SetGrowthStage` _returnvalue 0)
    (set `self.SpawnedCrop` _returnvalue)
    (bind _returnvalue_2 (`KismetSystemLibrary.K2_SetTimer` null "OnGrowthTick" (/ _growthtime (`KismetArrayLibrary.Array_Length` _growthstagemeshes)) true))
    (set `self.GrowthTimer` _returnvalue_2)))

(event `OnGrowthTick`
  (set `self.GrowthProgress` (`KismetMathLibrary.FClamp` (+ (`self.GrowthProgress`) 0.33)))
  (`/Game/FarmingGame/CaraFolder/Grass-Dirt-Farmland/Crop_BP.SetGrowthStage` (`self.SpawnedCrop`) (`KismetMathLibrary.FFloor` (* (`self.GrowthProgress`) (- (`KismetArrayLibrary.Array_Length` (`.GrowthStageMeshes` (defaults `Object` (`self.CurrentSeed`)))) 1))))
  (if (>= (`self.GrowthProgress`) 1.0)
    (`KismetSystemLibrary.K2_ClearAndInvalidateTimerHandle` (`self.GrowthTimer`))
    (set `self.FarmlandState` "NewEnumerator2")))

(event `Harvest`
  (params (ItemData :type "/Game/FarmingGame/AnthonyFolder/Items/ItemBP/BP_BaseItem Class Reference"))
  (if (== ItemData "/Game/FarmingGame/AnthonyFolder/Items/ItemBP/BP_Tool_Hoe.BP_Tool_Hoe_C")
    (`KismetSystemLibrary.K2_ClearAndInvalidateTimerHandle` (`self.GrowthTimer`))
    (`|SpawnActorFromClass` (`.HarvestItemClass` (defaults `Object` (`self.CurrentSeed`))) (`KismetMathLibrary.MakeTransform` (+ (`self.K2_GetActorLocation`) (0.0 0.0 100.0))) "Undefined" "MultiplyWithRoot" null null)
    (`self.K2_DestroyActor` (`self.SpawnedCrop`))
    (set `self.SpawnedCrop` null)
    (set `self.GrowthProgress` 0.0)
    (set `self.CurrentSeed` null)
    (set `self.FarmlandState` "NewEnumerator0")))

(fn `UserConstructionScript`)