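; BP_ItemPickup is a world item that adds its ItemData to the hotbar of an overlapping actor with a BPC_Inventory component.
; On BeginPlay, a random angular impulse spins its mesh.
; Overlap triggers Pickup immediately if CanPickup is set; otherwise a short delay enables it and retries.
; Pickup confirms the stored actor still overlaps and destroys the item only when AddItemToHotbar succeeds.
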(event `self.ReceiveBeginPlay`
  (`self.AddRandomRotation`))

(event `self.ReceiveActorBeginOverlap`
  (params (OtherActor :type "Actor Object Reference"))
  ; Detect character for pickup
  (set `self.OverlappingActor` OtherActor)
  (if (`self.CanPickup`)
    (`self.Pickup`)
    (else
      (`self.Cooldown`))))

(event `Cooldown`
  ; If cannot pickup enable after delay then attempt to try to pickup
  (`KismetSystemLibrary.Delay` 2.0)
  (set `self.CanPickup` true)
  (`self.Pickup`))

(fn `AddRandomRotation`
  (`PrimitiveComponent.AddAngularImpulseInDegrees` (`self.Mesh`) (* (`KismetMathLibrary.RandomUnitVector`) (`KismetMathLibrary.Conv_DoubleToVector` 350.0)) "None" true))

(fn `Pickup`
  (bind _returnvalue (`self.GetComponentByClass` (`self.OverlappingActor`) "/Game/FarmingGame/AnthonyFolder/BPC_Inventory.BPC_Inventory_C"))
  ; Verifies character attempting to pickup has inventory and currently still overlapping with it
  (if (`self.CanPickup`)
    (`/Engine/EditorBlueprintResources/StandardMacros.IsValid` _returnvalue
      (:`Is Valid`
        (if (`self.IsOverlappingActor` (`self.OverlappingActor`))
          (bind _itemadded (`/Game/FarmingGame/AnthonyFolder/BPC_Inventory.AddItemToHotbar` _returnvalue (`self.ItemData`)))
          (if _itemadded
            (`self.K2_DestroyActor`)))))))

(fn `UserConstructionScript`)