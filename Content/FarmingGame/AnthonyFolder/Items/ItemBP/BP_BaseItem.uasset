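; BP_BaseItem is a base item for the farming game, providing tool-style Attack and Interact actions on a hit actor.
; Both actions call ToggleAction, which plays the item action montage at double speed on the owner's skeletal mesh.
; If the target has the interface, they send it a tool attack or interact message with the item's class and inventory.
; Otherwise they only print debug text.
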(event `ToggleAction`
  (bind _returnvalue (`self.GetComponentByClass` (`self.GetOwner`) "/Script/Engine.SkeletalMeshComponent"))
  (`/Engine/EditorBlueprintResources/StandardMacros.IsValid` _returnvalue
    (:`Is Valid`
      (`|PlayMontage` _returnvalue "/Game/FarmingGame/AnthonyFolder/Animations/AM_ItemAction.AM_ItemAction" 2.0))))

(fn `Attack`
  (params (HitActor :type "Actor Object Reference") (DoesHitContainInterface :type Boolean) (Inventory :type "/Game/FarmingGame/AnthonyFolder/BPC_Inventory Object Reference"))
  (`self.ToggleAction`)
  (if DoesHitContainInterface
    (message `/Game/FarmingGame/AnthonyFolder/BPI_ItemAction.OnToolAttack` HitActor (`GameplayStatics.GetObjectClass` self) Inventory)
    (else
      (`KismetSystemLibrary.PrintString` "No action interface found :("))))

(fn `Interact`
  (params (HitActor :type "Actor Object Reference") (DoesHitContainInterface :type Boolean) (Inventory :type "/Game/FarmingGame/AnthonyFolder/BPC_Inventory Object Reference"))
  (`self.ToggleAction`)
  (if DoesHitContainInterface
    (message `/Game/FarmingGame/AnthonyFolder/BPI_ItemAction.OnToolInteract` HitActor (`GameplayStatics.GetObjectClass` self) Inventory)
    (else
      (`KismetSystemLibrary.PrintString` (`KismetSystemLibrary.GetDisplayName` HitActor)))))

(fn `UserConstructionScript`)