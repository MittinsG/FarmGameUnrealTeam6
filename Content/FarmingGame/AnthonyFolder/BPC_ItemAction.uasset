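; Actor component that provides an eye-level line trace for item actions, finding the actor a held or used item targets.
; On BeginPlay it caches its owning Character.
; RayCast traces on Visibility from the mesh "eyes" socket along the view rotation for the item's TraceDistance, ignoring character and item.
; It returns the hit actor and whether it implements BPI_ItemAction, without invoking the action itself.
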(event `self.ReceiveBeginPlay`
  (bind _ascharacter (cast `Character` (`self.GetOwner`)))
  (set `self.character` _ascharacter))

(fn `RayCast`
  (params (Item :type "/Game/FarmingGame/AnthonyFolder/Items/ItemBP/BP_BaseItem Object Reference"))
  (returns (HitActor :type "Actor Object Reference") (DoesHitContainInterface :type Boolean))
  (bind _character (`self.character`))
  (bind _returnvalue (`SceneComponent.GetSocketLocation` (`Character.Mesh` _character) "eyes"))
  ; Makes line trace from actor eyes and checks if it has action interface
  (`/Engine/EditorBlueprintResources/StandardMacros.IsValid` _character
    (:`Is Valid`
      (bind (_outhit _returnvalue_2) (`KismetSystemLibrary.LineTraceSingle` _returnvalue (+ _returnvalue (* (`KismetMathLibrary.GetForwardVector` (`.OutRotation` (`Actor.GetActorEyesViewPoint` _character))) (`/Game/FarmingGame/AnthonyFolder/Items/ItemBP/BP_BaseItem.TraceDistance` Item))) "TraceTypeQuery1" true (`|MakeArray` _character Item :!type "Actor Object Reference")))
      (if _returnvalue_2
        (bind (_bblockinghit _binitialoverlap _time _distance _location _impactpoint _normal _impactnormal _physmat _hitactor) (`GameplayStatics.BreakHitResult` _outhit))
        (return _hitactor (`KismetSystemLibrary.DoesImplementInterface` _hitactor "/Game/FarmingGame/AnthonyFolder/BPI_ItemAction.BPI_ItemAction_C"))
        (else
          (return null false))))
    (:`Is Not Valid`
      (`KismetSystemLibrary.PrintString` "No valid owner attatched to item for line trace"))))